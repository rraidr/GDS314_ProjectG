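; BP_Bullet_Particle_Enemies is a projectile actor, by its name an enemy bullet, that can re-aim and home on a target.
; LockOn turns it toward HitLocation and rebuilds its velocity along the new facing at the same speed.
; Each tick copies its HomingTargetComponent variable into the ProjectileMovement component.
; Any hit on its static mesh destroys the actor, with no damage handling in its graphs.
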(event OnComponentHit(StaticMesh)
  (params (HitComponent :type Primitive%20Component%20Object%20Reference) (OtherActor :type Actor%20Object%20Reference) (OtherComp :type Primitive%20Component%20Object%20Reference) (NormalImpulse :type Vector :default "0, 0, 0") (Hit :type Hit%20Result%20Structure%20%28by%20ref%29))
  (Actor|DestroyActor))

(event Custom|LockOn
  (bind _returnvalue (Transformation|GetActorRotation))
  (Transformation|SetActorRotation (Math|Rotator|FindLookatRotation (Transformation|GetActorLocation) (Variables|Default|GetHit%20Location)))
  (Variables|/Script/Engine.MovementComponent|SetVelocity (Variables|Default|GetProjectileMovement) (Class|KismetMathLibrary|CreateVectorfromYawPitch (.yaw _returnvalue) (.pitch _returnvalue) (Math|Vector|VectorLength (Transformation|GetVelocity)))))

(event EventTick
  (params (DeltaSeconds :type Float%20%28single-precision%29))
  (Variables|/Script/Engine.ProjectileMovementComponent|SetHomingTargetComponent (Variables|Default|GetProjectileMovement) (Variables|Default|GetHoming%20Target%20Component)))

(fn ConstructionScript)