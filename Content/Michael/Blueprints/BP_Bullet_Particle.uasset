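; BP_Bullet_Particle is a projectile bullet that aims itself at the player character's HitLocation when it spawns.
; On BeginPlay it copies that location from BP_Player_Character and calls LockOn once, so it does not track afterward.
; LockOn rotates the actor toward the point and redirects ProjectileMovement velocity along that rotation, preserving speed.
; The actor destroys itself when the Bullet component hits something, with no damage logic in its graphs.
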(event OnComponentHit(Bullet)
  (params (HitComponent :type Primitive%20Component%20Object%20Reference) (OtherActor :type Actor%20Object%20Reference) (OtherComp :type Primitive%20Component%20Object%20Reference) (NormalImpulse :type Vector :default "0, 0, 0") (Hit :type Hit%20Result%20Structure%20%28by%20ref%29))
  (Actor|DestroyActor))

(event Custom|LockOn
  (bind _returnvalue (Transformation|GetActorRotation))
  (Transformation|SetActorRotation (Math|Rotator|FindLookatRotation (Transformation|GetActorLocation) (Variables|Default|GetHit%20Location)))
  (Variables|/Script/Engine.MovementComponent|SetVelocity (Variables|Default|GetProjectileMovement) (Class|KismetMathLibrary|CreateVectorfromYawPitch (.yaw _returnvalue) (.pitch _returnvalue) (Math|Vector|VectorLength (Transformation|GetVelocity)))))

(event EventBeginPlay
  (bind _asbp_player_character (Utilities|Casting|CastToBP_Player_Character (Game|GetPlayerCharacter 0)))
  (Variables|Default|SetAs%20BP%20Player%20Character _asbp_player_character)
  (Variables|Default|SetHit%20Location (Variables|/Game/Michael/Blueprints/BP_Player_Character.BP_Player_Character_C|GetHit%20Location _asbp_player_character))
  (CallFunction|Lockon))

(fn ConstructionScript)