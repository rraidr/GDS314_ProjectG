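; Blood particle projectile that homes in on the player character.
; Every 0.2 seconds from BeginPlay, LockOn enables homing and sets the target from FindHomingTarget.
; That function returns a player scene component only when the head socket is nearer than the stored closest distance, which it then updates.
; Sphere overlap destroys the particle if its OverlappedComponent, rather than the other component, equals the player mesh.
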(event OnComponentBeginOverlap(Sphere)
  (params (OverlappedComponent :type Primitive%20Component%20Object%20Reference) (OtherActor :type Actor%20Object%20Reference) (OtherComp :type Primitive%20Component%20Object%20Reference) (OtherBodyIndex :type Integer) (bFromSweep :type Boolean) (SweepResult :type Hit%20Result%20Structure%20%28by%20ref%29))
  (if (== OverlappedComponent (Variables|Default|GetMesh))
    (Actor|DestroyActor)))

(event Custom|LockOn
  (bind _projectilemovement (Variables|Default|GetProjectileMovement))
  (bind _homing_target (CallFunction|FindHomingTarget))
  (Variables|/Script/Engine.ProjectileMovementComponent|SetHomingTargetComponent _projectilemovement _homing_target)
  (Variables|/Script/Engine.ProjectileMovementComponent|SetbIsHomingProjectile _projectilemovement true))

(event EventBeginPlay
  (bind _asbp_player_character (Utilities|Casting|CastToBP_Player_Character (Game|GetPlayerCharacter 0)))
  (Variables|Default|SetMesh (Variables|/Script/Engine.Character|GetMesh _asbp_player_character))
  (CallFunction|Lockon :!label _label)
  (Utilities|FlowControl|Delay 0.2)
  (goto _label))

(event Collision|EventActorBeginOverlap
  (params (OtherActor :type Actor%20Object%20Reference)))

(event EventTick
  (params (DeltaSeconds :type Float%20%28single-precision%29)))

(fn ConstructionScript)

(fn FindHomingTarget
  (bind _asbp_player_character (Utilities|Casting|CastToBP_Player_Character (Game|GetPlayerCharacter 0)))
  (if (< (Math|Vector|VectorLength (- (Transformation|GetSocketLocation (Variables|/Script/Engine.Character|GetMesh _asbp_player_character) "head") (Transformation|GetActorLocation))) (Variables|Default|GetClosest%20Distance))
    (Variables|Default|SetClosest%20Distance (Math|Vector|VectorLength (- (Transformation|GetSocketLocation (Variables|/Script/Engine.Character|GetMesh _asbp_player_character) "head") (Transformation|GetActorLocation))))
    (bind _output_get (Variables|Default|SetAs%20BP%20Player%20Character _asbp_player_character))
    (return (Actor|GetComponentbyClass _output_get "/Script/Engine.SceneComponent"))))