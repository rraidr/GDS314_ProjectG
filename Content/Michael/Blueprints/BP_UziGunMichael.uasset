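; BP_UziGunMichael is an Uzi gun Blueprint that plays a reload animation when the player character is reloading.
; BeginPlay caches the player character and copies its Reloading flag.
; Tick polls the character's flag and, through a DoOnce gate, plays the non-looping animation on the SKSMG11X mesh.
; After a fixed delay it clears only its own Reloading copy and resets the gate.
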(event EventBeginPlay
  (bind _asbp_player_character (Utilities|Casting|CastToBP_Player_Character (Game|GetPlayerCharacter 0)))
  (bind _output_get (Variables|Default|SetAs%20BP%20Player%20Character _asbp_player_character))
  (Variables|Default|SetReloading (Variables|/Game/Michael/Blueprints/BP_Player_Character.BP_Player_Character_C|GetReloading _output_get)))

(event Collision|EventActorBeginOverlap
  (params (OtherActor :type Actor%20Object%20Reference)))

(event EventTick
  (params (DeltaSeconds :type Float%20%28single-precision%29))
  (if (Variables|/Game/Michael/Blueprints/BP_Player_Character.BP_Player_Character_C|GetReloading (Variables|Default|GetAs%20BP%20Player%20Character))
    (Utilities|FlowControl|DoOnce false :!label _label
      (:Completed
        (Components|Animation|PlayAnimation (Variables|Default|GetSK_SMG11_X) "/Game/Blueprints/UziGun/Anim/UziGunReloadAnim.UziGunReloadAnim" false)
        (Utilities|FlowControl|Delay 2.0)
        (Variables|Default|SetReloading false)
        (goto _label Reset)))))

(fn ConstructionScript)