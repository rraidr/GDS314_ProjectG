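; BP_Blood_Bomb is a sticky timed bomb that explodes three seconds after it begins play.
; On a static mesh hit, it attaches itself to the hit actor, keeping its world transform, unless that actor is tagged "Not Stickable".
; A particle effect activates shortly after spawn.
; The detonation timer spawns a BP_Explosion at the bomb's transform, then destroys the bomb.
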(event OnComponentHit(StaticMesh)
  (params (HitComponent :type Primitive%20Component%20Object%20Reference) (OtherActor :type Actor%20Object%20Reference) (OtherComp :type Primitive%20Component%20Object%20Reference) (NormalImpulse :type Vector :default "0, 0, 0") (Hit :type Hit%20Result%20Structure%20%28by%20ref%29))
  (if (not (Actor|ActorHasTag (.hitactor Hit) "Not Stickable"))
    (Transformation|AttachActorToActor (.hitactor Hit) "None" "KeepWorld" "KeepWorld" "KeepWorld" true)
    (Development|PrintString "Stuck")))

(event Custom|Detonate
  (Game|SpawnActorfromClass "/Game/Michael/Blueprints/BP_Explosion.BP_Explosion_C" (Transformation|GetActorTransform) "Undefined" 0 0)
  (Actor|DestroyActor))

(event EventBeginPlay
  (Utilities|Time|SetTimerbyEvent (delegate Custom|Detonate) 3.0)
  (Utilities|FlowControl|Delay 0.3)
  (Components|Activation|Activate (Variables|Default|Getparticle%201) false))

(fn ConstructionScript)