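; BP_Explosion is a one-shot explosion actor that does all its work on BeginPlay.
; It fires a radial force impulse, sets its lifespan and applies radial damage credited to player controller 0, with equal inner and outer radii.
; Three particle emitters spawn at the force and sphere locations, two raised above them.
; An unconnected sphere-trace path applying point damage with BP_DT_Explosion never runs.
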(event EventBeginPlay
  (Class|RadialForceComponent|FireImpulse (Variables|Default|GetRadialForce))
  (Actor|SetLifeSpan (Variables|Default|GetIn%20Lifespan))
  (Class|GameplayStatics|ApplyRadialDamagewithFalloff (Variables|Default|GetBase%20Damage) 1e+02 (Transformation|GetWorldLocation (Variables|Default|GetSphere)) 5e+02 5e+02 0.0 0 0 self (Game|GetPlayerController 0) "ECC_GameTraceChannel3")
  (Effects|SpawnEmitteratLocation "/Game/FluidNinja/Input/FluidPresets/Explosion/PS_Explosion8Michael.PS_Explosion8Michael" (+ (Transformation|GetWorldLocation (Variables|Default|GetRadialForce)) "0,0.000000,90.000000"))
  (Effects|SpawnEmitteratLocation "/Game/FluidNinja/Input/FluidPresets/Explosion/PS_Explosion9Michael.PS_Explosion9Michael" (+ (Transformation|GetWorldLocation (Variables|Default|GetSphere)) "0,0.000000,350.000000"))
  (Effects|SpawnEmitteratLocation "/Game/FluidNinja/Usecases/Particles/PS_FluidNinja_VectorField_Pyro3FlameMichael.PS_FluidNinja_VectorField_Pyro3FlameMichael" (Transformation|GetWorldLocation (Variables|Default|GetSphere))))

(fn ConstructionScript)