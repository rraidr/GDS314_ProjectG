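; BP_AI_Test is a test AI character that takes point, radial and explosion damage and ragdolls on death.
; Hits subtract and print health, with point and explosion-type hits also playing a hit reaction and bullet hits spawning blood.
; When health drops below one, it simulates physics from the pelvis down, disables movement and applies a directional impulse.
; While dead, Tick keeps the collision-disabled capsule following the pelvis socket.
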(event EventBeginPlay
  (bind _asbp_player_character (Utilities|Casting|CastToBP_Player_Character (Game|GetPlayerCharacter 0)))
  (Variables|Default|SetAs%20BP%20Player%20Character _asbp_player_character))

(event Game|Damage|EventRadialDamage
  (params (DamageReceived :type Float%20%28single-precision%29) (DamageType :type Damage%20Type%20Object%20Reference) (Origin :type Vector :default "0, 0, 0") (HitInfo :type Hit%20Result%20Structure%20%28by%20ref%29) (InstigatedBy :type Controller%20Object%20Reference) (DamageCauser :type Actor%20Object%20Reference))
  (bind _output_get (Variables|Default|SetHealth (- (Variables|Default|GetHealth) DamageReceived)))
  (Development|PrintString (Utilities|String|ToString(Float) _output_get))
  (Utilities|IfDead)
  (Variables|Default|SetDead? true)
  (CallFunction|RagdollFunction)
  (Physics|AddImpulse (Variables|Character|GetMesh) (* (Math|Vector|GetForwardVector (Math|Rotator|FindLookatRotation Origin (Transformation|GetActorLocation))) 1e+04) "None" true))

(event EventTick
  (params (DeltaSeconds :type Float%20%28single-precision%29))
  ;[1 1 1] Setting Capsule Location
  (if (Variables|Default|GetDead?)
    (Transformation|SetWorldLocation (Variables|Collision|GetCapsuleComponent) (+ (Transformation|GetSocketLocation (Variables|Character|GetMesh) "pelvis") "0, 0,97.000000") false false)))

(event Game|Damage|EventPointDamage
  (params (Damage :type Float%20%28single-precision%29) (DamageType :type Damage%20Type%20Object%20Reference) (HitLocation :type Vector :default "0, 0, 0") (HitNormal :type Vector :default "0, 0, 0") (HitComponent :type Primitive%20Component%20Object%20Reference) (BoneName :type Name :default "None") (ShotFromDirection :type Vector :default "0, 0, 0") (InstigatedBy :type Controller%20Object%20Reference) (DamageCauser :type Actor%20Object%20Reference) (HitInfo :type Hit%20Result%20Structure%20%28by%20ref%29))
  ;[1 1 1] Damage
  (bind _output_get (Variables|Default|SetDamage%20Type DamageType))
  (if (not (== (Utilities|GetClass _output_get) "/Game/Michael/Blueprints/BP_DT_Explosion.BP_DT_Explosion_C"))
    (bind _output_get_2 (Variables|Default|SetHealth (- (Variables|Default|GetHealth) Damage)))
    (Development|PrintString (Utilities|String|ToString(Float) _output_get_2))
    (Components|Animation|PlayAnimation (Variables|Character|GetMesh) "/Game/AnimStarterPack/Hit_React_2.Hit_React_2" false)
    (Effects|SpawnEmitteratLocation "/Game/FXVillesBloodVFXPack/Particles/Cascade/Real/P_Blood_BulletHit.P_Blood_BulletHit" HitLocation)
    (Utilities|IfDead)
    (Variables|Default|SetDead? true)
    (CallFunction|RagdollFunction)
    (Physics|AddImpulseatLocation (Variables|Character|GetMesh) (* (Math|Vector|Normalize (- HitLocation ShotFromDirection)) 1e+04) HitLocation BoneName)
    (else
      (Utilities|ExplosionImpulse ShotFromDirection Damage))))

(fn ConstructionScript)

(fn RagdollFunction
  (bind _returnvalue (Utilities|Name|MakeLiteralName "pelvis"))
  (bind _mesh (Variables|Character|GetMesh))
  (Collision|SetCollisionEnabled (Variables|Collision|GetCapsuleComponent) "NoCollision")
  (Class|SkeletalMeshComponent|SetAllBodiesBelowSimulatePhysics _mesh _returnvalue true true)
  (Class|SkeletalMeshComponent|SetAllBodiesBelowPhysicsBlendWeight _mesh _returnvalue 0.8 false true)
  (Pawn|Components|CharacterMovement|DisableMovement (Variables|Character|GetCharacterMovement)))