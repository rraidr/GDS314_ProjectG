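; Enemy AI character that shoots, takes cover to reload and can be blood-bent or drained by health loss.
; A five-second firing timer flags OutofAmmo on the Blackboard, cleared by reloading in crouched cover.
; FireWeapon traces from the head along control rotation, applies point damage and spawns bullet particles from the gun tip.
; Damage handlers play hit reactions or blood effects, then ragdoll dead enemies with directional impulses and drop the weapon.
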(event OnComponentBeginOverlap(ExecuteCollider)
  (params (OverlappedComponent :type Primitive%20Component%20Object%20Reference) (OtherActor :type Actor%20Object%20Reference) (OtherComp :type Primitive%20Component%20Object%20Reference) (OtherBodyIndex :type Integer) (bFromSweep :type Boolean) (SweepResult :type Hit%20Result%20Structure%20%28by%20ref%29))
  ;[1 1 1] Executions
  (bind _asbp_player_character (Utilities|Casting|CastToBP_Player_Character OtherActor)))

(event Custom|Start%20Shooting
  ;[1 1 1] Shooting / Reloading
  (Variables|Default|SetAlerted? true)
  (Variables|Default|SetEnemyShoot? true)
  (Utilities|FlowControl|Delay 5.0)
  (Utilities|FlowControl|DoOnce false
    (:Completed
      (bind _output_get (Variables|Default|SetOutofAmmo true))
      (AI|Components|Blackboard|SetValueasBool (AI|GetBlackboard 0) (Utilities|Name|MakeLiteralName "OutofAmmo") _output_get))))

(event Custom|Stop%20Shooting
  ;[1 1 1] Shooting / Reloading
  (Variables|Default|SetEnemyShoot? false))

(event Custom|Execute
  ;[1 1 1] Executions
)

(event Custom|EnterCover
  ;[1 1 1] Look for Cover
  (Variables|Default|SetIsInCover true)
  (Variables|Default|SetEnemyShoot? false)
  (Character|Crouch)
  (CallFunction|Reloading))

(event Custom|Reloading
  (bind _returnvalue (Utilities|Name|MakeLiteralName "OutofAmmo"))
  (bind _returnvalue_2 (AI|GetBlackboard 0))
  ;[1 1 1] Shooting / Reloading
  (Variables|Default|SetReload? true)
  (Utilities|FlowControl|Delay 2.1)
  (Variables|Default|SetReload? false)
  (bind _output_get (Variables|Default|SetOutofAmmo false))
  (AI|Components|Blackboard|SetValueasBool _returnvalue_2 _returnvalue _output_get)
  (Utilities|FlowControl|DoOnce false) ; enters at Reset
)

(event Game|Damage|EventRadialDamage
  (params (DamageReceived :type Float%20%28single-precision%29) (DamageType :type Damage%20Type%20Object%20Reference) (Origin :type Vector :default "0, 0, 0") (HitInfo :type Hit%20Result%20Structure%20%28by%20ref%29) (InstigatedBy :type Controller%20Object%20Reference) (DamageCauser :type Actor%20Object%20Reference))
  ;[1 1 1] Radial damage
  (bind _output_get (Variables|Default|SetHealth (- (Variables|Default|GetHealth) DamageReceived)))
  (Development|PrintString (Utilities|String|ToString(Float) _output_get))
  (Utilities|IfDead)
  (Variables|Default|SetDead? true)
  (CallFunction|RagdollFunction)
  (Physics|AddImpulse (Variables|Character|GetMesh) (* (Math|Vector|GetForwardVector (Math|Rotator|FindLookatRotation Origin (Transformation|GetActorLocation))) 1e+04) "None" true))

(event EventTick
  (params (DeltaSeconds :type Float%20%28single-precision%29))
  (bind _ps (Variables|Default|GetPS))
  ;[1 1 1] Setting Capsule Location
  (if (Variables|Default|GetBloodBend?)
    (Utilities|FlowControl|DoOnce false :!label _label
      (:Completed
        (Components|Activation|Activate _ps false)
        (goto _label_2 Reset)))
    (else
      (Utilities|FlowControl|DoOnce false :!label _label_2
        (:Completed
          (Components|Activation|Deactivate _ps)
          (goto _label Reset))))))

(event Game|Damage|EventPointDamage
  (params (Damage :type Float%20%28single-precision%29) (DamageType :type Damage%20Type%20Object%20Reference) (HitLocation :type Vector :default "0, 0, 0") (HitNormal :type Vector :default "0, 0, 0") (HitComponent :type Primitive%20Component%20Object%20Reference) (BoneName :type Name :default "None") (ShotFromDirection :type Vector :default "0, 0, 0") (InstigatedBy :type Controller%20Object%20Reference) (DamageCauser :type Actor%20Object%20Reference) (HitInfo :type Hit%20Result%20Structure%20%28by%20ref%29))
  ;[1 1 1] Point Damage
  (bind _output_get (Variables|Default|SetDamage%20Type DamageType))
  (if (not (== (Utilities|GetClass _output_get) "/Game/Michael/Blueprints/BP_DT_Explosion.BP_DT_Explosion_C"))
    (bind _output_get_2 (Variables|Default|SetHealth (- (Math|Float|Clamp(Float) (Variables|Default|GetHealth) 15.0 1e+02) Damage)))
    (Development|PrintString (Utilities|String|ToString(Float) _output_get_2))
    (Variables|Default|SetHit? true)
    (Animation|PlayAnimMontage (Utilities|Select :Index (Math|Random|RandomInteger 3) :Option%200 "/Game/Characters/Enemy1/Anims/React/Hit_React_1_Montage.Hit_React_1_Montage" :Option%201 "/Game/Characters/Enemy1/Anims/React/Hit_React_2_Montage.Hit_React_2_Montage" :Option%202 "/Game/Characters/Enemy1/Anims/React/Hit_React_3_Montage.Hit_React_3_Montage" :Option%203 "/Game/Characters/Enemy1/Anims/React/Hit_React_4_Montage.Hit_React_4_Montage") 1.0 "None")
    (Effects|SpawnEmitteratLocation (.OutItem (Utilities|Array|Random (Utilities|Array|MakeArray "/Game/FXVillesBloodVFXPack/Particles/Cascade/Real/P_Blood_Spurt_01.P_Blood_Spurt_01" "/Game/FXVillesBloodVFXPack/Particles/Cascade/Real/P_Blood_Spurt_Small.P_Blood_Spurt_Small" "/Game/FXVillesBloodVFXPack/Particles/Cascade/Real/P_Blood_Spurt_02.P_Blood_Spurt_02" "/Game/FXVillesBloodVFXPack/Particles/Cascade/Real/P_Blood_Burst_Omni.P_Blood_Burst_Omni" "/Game/FXVillesBloodVFXPack/Particles/Cascade/Real/P_Blood_BulletHit.P_Blood_BulletHit"))) HitLocation)
    (Utilities|FlowControl|Sequence
      (:then_0
        (Utilities|FlowControl|Delay 0.5)
        (Variables|Default|SetHit? false)
        (Components|Animation|SetAnimationMode (Variables|Character|GetMesh) "AnimationBlueprint")
        (Utilities|IfDead)
        (Variables|Default|SetDead? true)
        (CallFunction|RagdollFunction)
        (Physics|AddImpulseatLocation (Variables|Character|GetMesh) (* (Math|Vector|Normalize (- HitLocation ShotFromDirection)) 1e+04) HitLocation BoneName)))
    (else
      (Utilities|ExplosionImpulse ShotFromDirection Damage))))

(fn ConstructionScript)

(fn RagdollFunction
  (bind _returnvalue (Utilities|Name|MakeLiteralName "cc_base_hip"))
  (bind _mesh (Variables|Character|GetMesh))
  (bind _weapon (Variables|Default|GetWeapon))
  (Collision|SetCollisionEnabled (Variables|Collision|GetCapsuleComponent) "NoCollision")
  (Class|SkeletalMeshComponent|SetAllBodiesBelowSimulatePhysics _mesh _returnvalue true true)
  (Class|SkeletalMeshComponent|SetAllBodiesBelowPhysicsBlendWeight _mesh _returnvalue 0.8 false true)
  (Pawn|Components|CharacterMovement|DisableMovement (Variables|Character|GetCharacterMovement))
  (Collision|SetCollisionProfileName (Variables|Character|GetMesh) "DeathCollision" true :!class /Script/Engine.PrimitiveComponent)
  (Transformation|DetachFromComponent _weapon "KeepWorld" "KeepWorld" "KeepWorld" true)
  (Collision|SetCollisionEnabled _weapon "PhysicsOnly")
  (Physics|SetSimulatePhysics _weapon true))

(fn FireWeapon
  (bind _gun_tip (Variables|Default|GetGun%20Tip))
  (bind _mesh (Variables|Character|GetMesh))
  (bind _returnvalue (Transformation|GetSocketLocation _mesh "cc_base_head"))
  (bind _returnvalue_2 (Transformation|GetWorldLocation _gun_tip))
  ;[1 1 1] Trace and apply damage
  (bind (_location _hit_info _hit_actor _rotation _hitcomponent _hitbonename _impactpoint) (Utilities|LineTrace _returnvalue)
    (:Done
      (Variables|Default|SetHit%20Location _impactpoint)
      (Game|Damage|ApplyPointDamage _hit_actor (Variables|Default|GetCurrent%20Damage) _returnvalue _hit_info (Pawn|GetController) self)
      (Game|SpawnActorfromClass "/Game/Michael/Blueprints/BP_Bullet_Particle_Enemies.BP_Bullet_Particle_Enemies_C" (Math|Transform|MakeTransform _returnvalue_2 (Math|Rotator|FindLookatRotation _returnvalue_2 _impactpoint) "2.000000,2.000000,2.000000") "Undefined" 0 0)
      (if (Physics|IsSimulatingPhysics _hitcomponent _hitbonename)
        (Physics|SetPhysicsLinearVelocity _hitcomponent (* (Math|Vector|GetForwardVector (Transformation|GetWorldRotation (Variables|Default|GetGun%20Tip))) (Variables|Default|GetBulletforce)) true _hitbonename)))))

(fn Drain
  (Variables|Default|SetDrained? true)
  (Variables|Default|SetHealth (- (Variables|Default|GetHealth) 1e+02)))