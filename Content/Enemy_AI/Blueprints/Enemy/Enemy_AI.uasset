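; AI controller for patrolling enemies that runs the Enemy_BT behavior tree and reacts to the player.
; On BeginPlay it seeds the Blackboard from the pawn's patrol path and ammo state.
; Perception updates CanSeePlayer for the player, then passes through a DoOnce to write StopPatrol from the Alerted value and raise walk speed if sensed.
; HitReact enters that same alert logic directly, bypassing the DoOnce.
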(event OnTargetPerceptionUpdated(AIPerception)
  (params (Actor :type Actor%20Object%20Reference) (Stimulus :type AI%20Stimulus%20Structure))
  (bind _returnvalue (AI|GetBlackboard 0))
  (Utilities|Casting|CastToBP_Player_Character Actor)
  (AI|Components|Blackboard|SetValueasBool _returnvalue (Utilities|Name|MakeLiteralName "CanSeePlayer") (.bsuccessfullysensed Stimulus))
  (Utilities|FlowControl|DoOnce false
    (:Completed
      (AI|Components|Blackboard|SetValueasBool _returnvalue (Utilities|Name|MakeLiteralName "StopPatrol") (stale Custom|HitReact Alerted))
      (if (.bsuccessfullysensed Stimulus)
        (bind _asbp_enemy_ai (Utilities|Casting|CastToBP_Enemy_AI (Variables|Default|GetAs%20BP%20Enemy%20AI)))
        (Variables|/Script/Engine.CharacterMovementComponent|SetMaxWalkSpeed (Variables|/Script/Engine.Character|GetCharacterMovement _asbp_enemy_ai) 6e+02)))))

(event Custom|HitReact
  (params (Alerted :type Boolean))
  (AI|Components|Blackboard|SetValueasBool (AI|GetBlackboard 0) (Utilities|Name|MakeLiteralName "StopPatrol") Alerted)
  (if (.bsuccessfullysensed (stale OnTargetPerceptionUpdated(AIPerception) Stimulus))
    (bind _asbp_enemy_ai (Utilities|Casting|CastToBP_Enemy_AI (Variables|Default|GetAs%20BP%20Enemy%20AI)))
    (Variables|/Script/Engine.CharacterMovementComponent|SetMaxWalkSpeed (Variables|/Script/Engine.Character|GetCharacterMovement _asbp_enemy_ai) 6e+02)))

(event EventBeginPlay
  (bind _returnvalue (AI|GetBlackboard 0))
  (AI|RunBehaviorTree "/Game/Enemy_AI/Blueprints/Enemy/Enemy_BT.Enemy_BT")
  (bind _asbp_enemy_ai (Utilities|Casting|CastToBP_Enemy_AI (Pawn|GetControlledPawn)))
  (bind _output_get (Variables|Default|SetAs%20BP%20Enemy%20AI _asbp_enemy_ai))
  (AI|Components|Blackboard|SetValueasBool _returnvalue (Utilities|Name|MakeLiteralName "PathLooping") (Variables|/Game/Enemy_AI/Blueprints/Enemy/PatrolPath.PatrolPath_C|GetIsLooping (Variables|/Game/Enemy_AI/Blueprints/Enemy/BP_Enemy_AI.BP_Enemy_AI_C|GetPatrolPath _output_get)))
  (AI|Components|Blackboard|SetValueasFloat _returnvalue (Utilities|Name|MakeLiteralName "WaitTime") (Variables|/Game/Enemy_AI/Blueprints/Enemy/PatrolPath.PatrolPath_C|GetWaitTime (Variables|/Game/Enemy_AI/Blueprints/Enemy/BP_Enemy_AI.BP_Enemy_AI_C|GetPatrolPath _output_get)))
  (AI|Components|Blackboard|SetValueasBool _returnvalue (Utilities|Name|MakeLiteralName "OutofAmmo") (Variables|/Game/Enemy_AI/Blueprints/Enemy/BP_Enemy_AI.BP_Enemy_AI_C|GetOutofAmmo _asbp_enemy_ai))
  (Class|BlackboardComponent|SetValueasInt (AI|GetBlackboard 0) (Utilities|Name|MakeLiteralName "Direction") 1))

(fn ConstructionScript)