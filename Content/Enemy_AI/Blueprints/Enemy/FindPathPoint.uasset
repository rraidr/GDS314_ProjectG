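; FindPathPoint is a behavior tree task that gives an enemy AI its current patrol destination.
; It reads the path index from the blackboard, takes that point from the pawn's PatrolPath, converts it to world space and writes it to the path vector key.
; It finishes only on success, with no finish call when the cast fails or the path is invalid.
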(event EventReceiveExecuteAI
  (params (OwnerController :type AI%20Controller%20Object%20Reference) (ControlledPawn :type Pawn%20Object%20Reference))
  (bind _asbp_enemy_ai (Utilities|Casting|CastToBP_Enemy_AI ControlledPawn))
  (bind _patrolpath (Variables|/Game/Enemy_AI/Blueprints/Enemy/BP_Enemy_AI.BP_Enemy_AI_C|GetPatrolPath _asbp_enemy_ai)
    (:then
      (AI|BehaviorTree|SetBlackboardValueasVector (Variables|Default|GetBB_PathVector) (Math|Transform|TransformLocation (Transformation|GetActorTransform _patrolpath) (Utilities|Array|Get(acopy) (Variables|/Game/Enemy_AI/Blueprints/Enemy/PatrolPath.PatrolPath_C|GetPathPoints _patrolpath) (Class|BTFunctionLibrary|GetBlackboardValueasInt (Variables|Default|GetBB_PathIndex)))))
      (AI|BehaviorTree|FinishExecute true))
    (:else)))