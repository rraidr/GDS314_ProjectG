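; AI controller for enemies that patrol and react to seeing the player, driven by the Enemy_BT behavior tree.
; On BeginPlay it starts the tree and copies the controlled pawn's patrol path looping flag into the Blackboard.
; AI Perception updates for the player character keep CanSeePlayer current.
; A DoOnce with no reset writes StopPatrol only on the first such update.
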(event OnTargetPerceptionUpdated(AIPerception)
  (params (Actor :type Actor%20Object%20Reference) (Stimulus :type AI%20Stimulus%20Structure))
  (bind _returnvalue (AI|GetBlackboard 0))
  (Utilities|Casting|CastToBP_Player_Character Actor)
  (AI|Components|Blackboard|SetValueasBool _returnvalue (Utilities|Name|MakeLiteralName "CanSeePlayer") (.bsuccessfullysensed Stimulus))
  (Utilities|FlowControl|DoOnce false
    (:Completed
      (AI|Components|Blackboard|SetValueasBool _returnvalue (Utilities|Name|MakeLiteralName "StopPatrol") (.bsuccessfullysensed Stimulus)))))

(event EventBeginPlay
  (AI|RunBehaviorTree "/Game/Enemy_AI/Blueprints/Enemy_BT.Enemy_BT")
  (bind _asbp_enemy_ai (Utilities|Casting|CastToBP_Enemy_AI (Pawn|GetControlledPawn)))
  (bind _output_get (Variables|Default|SetAs%20BP%20Enemy%20AI _asbp_enemy_ai))
  (AI|Components|Blackboard|SetValueasBool (AI|GetBlackboard 0) (Utilities|Name|MakeLiteralName "PathLooping") (Variables|/Game/Enemy_AI/Blueprints/PatrolPath.PatrolPath_C|GetIsLooping (Variables|/Game/Enemy_AI/Blueprints/BP_Enemy_AI.BP_Enemy_AI_C|GetPatrolPath _output_get))))

(fn ConstructionScript)