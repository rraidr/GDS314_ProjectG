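; Boss enemy character with a timed charge attack, health and ragdoll death.
; While charging, capsule overlap with the player applies charge damage and sets the Blackboard "Hit" key.
; Player contact also toggles a CanBeDmg flag, cleared after a delay or on sphere exit.
; Point damage spawns random blood effects and triggers hip-down physics ragdoll at zero health, while radial damage only reduces health.
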(event OnComponentBeginOverlap(CapsuleComponent)
  (params (OverlappedComponent :type Primitive%20Component%20Object%20Reference) (OtherActor :type Actor%20Object%20Reference) (OtherComp :type Primitive%20Component%20Object%20Reference) (OtherBodyIndex :type Integer) (bFromSweep :type Boolean) (SweepResult :type Hit%20Result%20Structure%20%28by%20ref%29))
  ;[1 1 1] Hit Box / Charge DMG and Check
  (bind _asbp_player_character (Utilities|Casting|CastToBP_Player_Character OtherActor))
  (Variables|Default|SetCanBeDmg true)
  (if (Variables|Default|GetCharging?)
    (Game|Damage|ApplyDamage _asbp_player_character (Variables|Default|GetChargeDMG) 0 0)
    (AI|Components|Blackboard|SetValueasBool (AI|GetBlackboard 0) (Utilities|Name|MakeLiteralName "Hit") true)
    (Utilities|FlowControl|Delay 2.0)
    (Variables|Default|SetCanBeDmg false)
    (else
      (Utilities|FlowControl|Delay 2.0)
      (Variables|Default|SetCanBeDmg false))))

(event OnComponentEndOverlap(Sphere)
  (params (OverlappedComponent :type Primitive%20Component%20Object%20Reference) (OtherActor :type Actor%20Object%20Reference) (OtherComp :type Primitive%20Component%20Object%20Reference) (OtherBodyIndex :type Integer))
  ;[1 1 1] Hit Box / Charge DMG and Check
  (Utilities|Casting|CastToBP_Player_Character OtherActor)
  (Variables|Default|SetCanBeDmg false))

(event Custom|Charging
  ;[1 1 1] Charge Animation / Event
  (Components|Animation|SetAnimationMode (Variables|Character|GetMesh) "AnimationBlueprint")
  (Variables|Default|SetCharging? true)
  (Utilities|FlowControl|Delay 2.8)
  (Variables|Default|SetCharging? false))

(event Game|Damage|EventRadialDamage
  (params (DamageReceived :type Float%20%28single-precision%29) (DamageType :type Damage%20Type%20Object%20Reference) (Origin :type Vector :default "0, 0, 0") (HitInfo :type Hit%20Result%20Structure%20%28by%20ref%29) (InstigatedBy :type Controller%20Object%20Reference) (DamageCauser :type Actor%20Object%20Reference))
  (Variables|Default|SetHealth (- (Variables|Default|GetHealth) DamageReceived)))

(event Game|Damage|EventPointDamage
  (params (Damage :type Float%20%28single-precision%29) (DamageType :type Damage%20Type%20Object%20Reference) (HitLocation :type Vector :default "0, 0, 0") (HitNormal :type Vector :default "0, 0, 0") (HitComponent :type Primitive%20Component%20Object%20Reference) (BoneName :type Name :default "None") (ShotFromDirection :type Vector :default "0, 0, 0") (InstigatedBy :type Controller%20Object%20Reference) (DamageCauser :type Actor%20Object%20Reference) (HitInfo :type Hit%20Result%20Structure%20%28by%20ref%29))
  ;[1 1 1] Health / DMG
  (Variables|Default|SetHealth (- (Variables|Default|GetHealth) Damage))
  (Effects|SpawnEmitteratLocation (.OutItem (Utilities|Array|Random (Utilities|Array|MakeArray "/Game/FXVillesBloodVFXPack/Particles/Cascade/Real/P_Blood_Spurt_01.P_Blood_Spurt_01" "/Game/FXVillesBloodVFXPack/Particles/Cascade/Real/P_Blood_Spurt_02.P_Blood_Spurt_02" "/Game/FXVillesBloodVFXPack/Particles/Cascade/Real/P_Blood_Spurt_Small.P_Blood_Spurt_Small" "/Game/FXVillesBloodVFXPack/Particles/Cascade/Real/P_Blood_Burst_Omni.P_Blood_Burst_Omni" "/Game/FXVillesBloodVFXPack/Particles/Cascade/Real/P_Blood_BulletHit.P_Blood_BulletHit"))) HitLocation)
  (if (< (Variables|Default|GetHealth) 1.0)
    (CallFunction|Ragdoll)
    (Variables|Default|SetIsDead? true)))

(fn ConstructionScript)

(fn Ragdoll
  (bind _returnvalue (Utilities|Name|MakeLiteralName "Hips"))
  (bind _mesh (Variables|Character|GetMesh))
  (Collision|SetCollisionEnabled (Variables|Collision|GetCapsuleComponent) "NoCollision")
  (Class|SkeletalMeshComponent|SetAllBodiesBelowSimulatePhysics _mesh _returnvalue true true)
  (Class|SkeletalMeshComponent|SetAllBodiesBelowPhysicsBlendWeight _mesh _returnvalue 0.8 false true)
  (Pawn|Components|CharacterMovement|DisableMovement (Variables|Character|GetCharacterMovement))
  (Collision|SetCollisionProfileName (Variables|Character|GetMesh) "DeathCollision" true :!class /Script/Engine.PrimitiveComponent))