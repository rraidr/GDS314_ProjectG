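; Behavior tree task for the boss AI that performs a timed melee attack on the player.
; It plays a punch animation directly on the boss mesh, waits for the hit moment, and applies a small damage if the player overlaps the boss.
; After a second delay it restores the Animation Blueprint, clears the ChargeCooldown and Hit blackboard flags, and finishes successfully.
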(event EventReceiveExecuteAI
  (params (OwnerController :type AI%20Controller%20Object%20Reference) (ControlledPawn :type Pawn%20Object%20Reference))
  (bind _asbp_boss_ai (Utilities|Casting|CastToBP_Boss_AI ControlledPawn))
  (Components|Animation|PlayAnimation (Variables|/Script/Engine.Character|GetMesh _asbp_boss_ai) "/Game/Characters/Boss/Animations/Zombie_Punching.Zombie_Punching" false)
  (Utilities|FlowControl|Delay 1.2)
  ;[1 1 1] Applies DMG on Animation if Player is near
  (bind _asbp_player_character (Utilities|Casting|CastToBP_Player_Character (Game|GetPlayerCharacter 0)))
  (if (Collision|IsOverlappingActor _asbp_player_character _asbp_boss_ai :!class /Script/Engine.Actor)
    (Game|Damage|ApplyDamage _asbp_player_character 0.4 0 0))
  (Utilities|FlowControl|Delay 2.6)
  (Components|Animation|SetAnimationMode (Variables|/Script/Engine.Character|GetMesh _asbp_boss_ai) "AnimationBlueprint")
  (AI|Components|Blackboard|SetValueasBool (AI|GetBlackboard _asbp_boss_ai) (Utilities|Name|MakeLiteralName "ChargeCooldown") false)
  (AI|Components|Blackboard|SetValueasBool (AI|GetBlackboard _asbp_boss_ai) (Utilities|Name|MakeLiteralName "Hit") false)
  (AI|BehaviorTree|FinishExecute true))