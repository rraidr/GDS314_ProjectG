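; AI controller for the boss enemy that drives it through the Boss_BT behavior tree.
; BeginPlay starts the tree, caches the controlled BP_Boss_AI pawn, then seeds the direction, charge-cooldown and hit blackboard keys if that cast succeeds.
; AI Perception updates for the player character write the sensed state to CanSeePlayer on the blackboard.
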(event OnTargetPerceptionUpdated(AIPerception)
  (params (Actor :type Actor%20Object%20Reference) (Stimulus :type AI%20Stimulus%20Structure))
  ;[1 1 1] AI Perception
  (Utilities|Casting|CastToBP_Player_Character Actor)
  (AI|Components|Blackboard|SetValueasBool (AI|GetBlackboard 0) (Utilities|Name|MakeLiteralName "CanSeePlayer") (.bsuccessfullysensed Stimulus)))

(event EventBeginPlay
  (bind _returnvalue (AI|GetBlackboard 0))
  (AI|RunBehaviorTree "/Game/Enemy_AI/Blueprints/Boss/Boss_BT.Boss_BT")
  (bind _asbp_boss_ai (Utilities|Casting|CastToBP_Boss_AI (Pawn|GetControlledPawn)))
  (Variables|Default|SetAs%20BP%20Boss%20AI _asbp_boss_ai)
  (Class|BlackboardComponent|SetValueasInt _returnvalue (Utilities|Name|MakeLiteralName "Direction") 1)
  (AI|Components|Blackboard|SetValueasBool _returnvalue (Utilities|Name|MakeLiteralName "ChargeCooldown") false)
  (AI|Components|Blackboard|SetValueasBool _returnvalue (Utilities|Name|MakeLiteralName "Hit") false))

(fn ConstructionScript)