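; BP_SingleDoor is a door that the player can knock loose with a melee attack.
; Its mesh starts with physics off until a BP_Player_Character overlaps the Box with its Melee flag set.
; That overlap turns on physics and collision, fires a radial force impulse and spawns a metal destruction particle at Box1.
; An unconnected mesh-swap node never runs.
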(event OnComponentBeginOverlap(Box)
  (params (OverlappedComponent :type Primitive%20Component%20Object%20Reference) (OtherActor :type Actor%20Object%20Reference) (OtherComp :type Primitive%20Component%20Object%20Reference) (OtherBodyIndex :type Integer) (bFromSweep :type Boolean) (SweepResult :type Hit%20Result%20Structure%20%28by%20ref%29))
  (bind _asbp_player_character (Utilities|Casting|CastToBP_Player_Character OtherActor))
  (if (Variables|/Game/Michael/Blueprints/BP_Player_Character.BP_Player_Character_C|GetMelee? _asbp_player_character)
    (Physics|SetSimulatePhysics (Variables|Default|GetDoorMesh) true)
    (Collision|SetCollisionEnabled (Variables|Default|GetDoorMesh) "QueryAndPhysics")
    (Class|RadialForceComponent|FireImpulse (Variables|Default|GetRadialForce))
    (Effects|SpawnEmitteratLocation (Utilities|Array|Get(acopy) (Utilities|Array|MakeArray "/Game/Realistic_Starter_VFX_Pack_Vol2/Particles/Destruction/P_Destruction_Metal.P_Destruction_Metal" "/Game/Realistic_Starter_VFX_Pack/Particles/Hit/P_Metal.P_Metal")) (Transformation|GetWorldLocation (Variables|Default|GetBox1)) "0, 0, 0" "0.500000,0.500000,0.500000")))

(event EventBeginPlay
  (Physics|SetSimulatePhysics (Variables|Default|GetDoorMesh) false))

(fn ConstructionScript)