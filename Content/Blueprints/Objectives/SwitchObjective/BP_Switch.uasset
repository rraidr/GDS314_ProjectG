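; BP_Switch is a wall switch objective that the player activates by pressing E while inside its trigger box.
; Box overlap toggles input and a gate on the key, and shows a custom-depth stencil highlight while the switch is unused.
; Pressing E sets SwitchActivated and clears the highlight, then a DoOnce plays an attached button audio event and a brief spark emitter.
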(event OnComponentBeginOverlap(Box)
  (params (OverlappedComponent :type Primitive%20Component%20Object%20Reference) (OtherActor :type Actor%20Object%20Reference) (OtherComp :type Primitive%20Component%20Object%20Reference) (OtherBodyIndex :type Integer) (bFromSweep :type Boolean) (SweepResult :type Hit%20Result%20Structure%20%28by%20ref%29))
  (bind _sm_wallswitch_02 (Variables|Default|GetSM_WallSwitch_02))
  (bind _sm_wallswitch_02_2 (Variables|Default|GetSM_WallSwitch_02))
  (Utilities|Casting|CastToBP_Player_Character OtherActor)
  (Input|EnableInput (Game|GetPlayerController 0))
  (if (Variables|Default|GetSwitchActivated)
    (Utilities|FlowControl|Gate true) ; enters at Open
    (else
      (Rendering|SetRenderCustomDepth _sm_wallswitch_02_2 true)
      (Rendering|SetCustomDepthStencilValue _sm_wallswitch_02_2 2)
      (Utilities|FlowControl|Gate true) ; enters at Open
    )))

(event OnComponentEndOverlap(Box)
  (params (OverlappedComponent :type Primitive%20Component%20Object%20Reference) (OtherActor :type Actor%20Object%20Reference) (OtherComp :type Primitive%20Component%20Object%20Reference) (OtherBodyIndex :type Integer))
  (bind _sm_wallswitch_02 (Variables|Default|GetSM_WallSwitch_02))
  (bind _sm_wallswitch_02_2 (Variables|Default|GetSM_WallSwitch_02))
  (Utilities|Casting|CastToBP_Player_Character OtherActor)
  (Input|DisableInput (Game|GetPlayerController 0))
  (if (Variables|Default|GetSwitchActivated)
    (Utilities|FlowControl|Gate true) ; enters at Close
    (else
      (Rendering|SetRenderCustomDepth _sm_wallswitch_02_2 false)
      (Rendering|SetCustomDepthStencilValue _sm_wallswitch_02_2 0)
      (Utilities|FlowControl|Gate true) ; enters at Close
    )))

(event Input|KeyboardEvents|E
  (params (Key :type Key%20Structure))
  (bind _sm_wallswitch_02 (Variables|Default|GetSM_WallSwitch_02))
  (:Pressed
    (Utilities|FlowControl|Gate true
      (:Exit
        (Variables|Default|SetSwitchActivated true)
        (Rendering|SetRenderCustomDepth _sm_wallswitch_02 false)
        (Rendering|SetCustomDepthStencilValue _sm_wallswitch_02 0)
        (Utilities|FlowControl|DoOnce false
          (:Completed
            (Class|FMODBlueprintStatics|PlayEventAttached "/Game/FMOD/Events/3D_SFX/OfficeButton.OfficeButton" (Variables|Default|GetSM_WallSwitch_02) "None" "0, 0, 0" "KeepRelativeOffset")
            (bind _returnvalue (Effects|SpawnEmitteratLocation "/Game/Realistic_Starter_VFX_Pack_Vol2/Particles/Sparks/P_Sparks_C.P_Sparks_C" (Transformation|GetWorldLocation (Variables|Default|GetSM_WallSwitch_02)) "0, 0, 0" "0.200000,0.200000,0.200000"))
            (Utilities|FlowControl|Delay 1.0)
            (Components|DestroyComponent _returnvalue)))))))

(fn ConstructionScript)