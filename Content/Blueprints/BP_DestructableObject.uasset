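; BP_DestructableObject is a breakable prop that either explodes on fracture or can respawn afterward.
; At BeginPlay it caches its transform and destructible mesh, then briefly disables physics simulation and query collision.
; When fractured, explosive objects fire a radial impulse and apply radial damage without respawning.
; Others switch to physics-only collision, wait, then, if Respawn is set, clear and reassign the mesh at the saved transform and repeat the safe-collision delay.
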(event OnComponentFracture(DestructibleComponent)
  (params (HitPoint :type Vector%20%28by%20ref%29 :default "0, 0, 0") (HitDirection :type Vector%20%28by%20ref%29 :default "0, 0, 0"))
  (if (Variables|Default|GetExplosive?)
    (Class|RadialForceComponent|FireImpulse (Variables|Default|GetRadialForce))
    (Game|Damage|ApplyRadialDamage 5e+01 (Transformation|GetWorldLocation (Variables|Default|GetDestructibleComponent)) 3e+02 0 0 0 0 false "ECC_Visibility")
    (else
      (Collision|SetCollisionEnabled (Variables|Default|GetDestructibleComponent) "PhysicsOnly")
      (Utilities|FlowControl|Delay 3e+01)
      (CallFunction|RegenerateMesh))))

(event Custom|Safe%20Collision
  (bind _destructiblecomponent (Variables|Default|GetDestructibleComponent))
  (Physics|SetSimulatePhysics _destructiblecomponent false)
  (Collision|SetCollisionEnabled _destructiblecomponent "PhysicsOnly")
  (Utilities|FlowControl|Delay 1.0)
  (Physics|SetSimulatePhysics _destructiblecomponent true)
  (Collision|SetCollisionEnabled _destructiblecomponent "QueryAndPhysics"))

(event EventBeginPlay
  (bind _destructiblecomponent (Variables|Default|GetDestructibleComponent))
  (Variables|Default|SetRespawnLocation (Transformation|GetWorldTransform _destructiblecomponent))
  (bind _returnvalue (Class|DestructibleComponent|GetDestructibleMesh _destructiblecomponent))
  (Variables|Default|SetDestructibleMesh _returnvalue)
  (CallFunction|SafeCollision))

(fn ConstructionScript)

(fn RegenerateMesh
  (if (Variables|Default|GetRespawn?)
    (Class|DestructibleComponent|SetDestructibleMesh (Variables|Default|GetDestructibleComponent))
    (Transformation|SetWorldTransform (Variables|Default|GetDestructibleComponent) (Variables|Default|GetRespawnLocation) false true)
    (Class|DestructibleComponent|SetDestructibleMesh (Variables|Default|GetDestructibleComponent) (Variables|Default|GetDestructibleMesh))
    (CallFunction|SafeCollision)
    (return)))