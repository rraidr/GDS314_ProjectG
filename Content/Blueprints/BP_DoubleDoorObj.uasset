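; Double door actor that swings two door meshes open and closed through DoorOpen and DoorClose events, with no trigger logic of its own.
; Each event drives both leaves at once, setting each mesh's relative yaw from its own timeline track.
; Opening and closing use separate timelines, played from the start and reversed from the end respectively, so motion never resumes from the current angle.
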(event Custom|DoorClose
  (Utilities|FlowControl|Sequence
    (:then_0
      (bind _rotationtrack (Timeline|Timeline_1 ReverseFromEnd)
        (:Update
          (Transformation|SetRelativeRotation (Variables|Default|GetSM_Door06) (Math|Rotator|MakeRotator 0.0 0.0 _rotationtrack) false false))))
    (:then_1
      (bind _rotationtrack_2 (Timeline|Timeline_2 ReverseFromEnd)
        (:Update
          (Transformation|SetRelativeRotation (Variables|Default|GetSM_Door07) (Math|Rotator|MakeRotator 0.0 0.0 _rotationtrack_2) false false))))))

(event Custom|DoorOpen
  (Utilities|FlowControl|Sequence
    (:then_0
      (bind _rotationtrack (Timeline|DoorRotate PlayFromStart)
        (:Update
          (Transformation|SetRelativeRotation (Variables|Default|GetSM_Door06) (Math|Rotator|MakeRotator 0.0 0.0 _rotationtrack) false false))))
    (:then_1
      (bind _rotationtrack_2 (Timeline|Timeline_0 PlayFromStart)
        (:Update
          (Transformation|SetRelativeRotation (Variables|Default|GetSM_Door07) (Math|Rotator|MakeRotator 0.0 0.0 _rotationtrack_2) false false))))))

(event Collision|EventActorBeginOverlap
  (params (OtherActor :type Actor%20Object%20Reference)))

(event EventTick
  (params (DeltaSeconds :type Float%20%28single-precision%29)))

(fn ConstructionScript)